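; Interactable test cube that grants the player double jump with an explosion effect.
; The Interaction event runs once: it prints a debug string, sets CanDoubleJump on the ThirdPersonCharacter, plays an explosion sound and spawns an explosion emitter at the cube.
; A separate Interact function destroys the actor and returns false; visibility and destroy nodes in the event graph are left unconnected.
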(event EventBeginPlay)

(event Collision|EventActorBeginOverlap
  (params (OtherActor :type Actor%20Object%20Reference)))

(event EventTick
  (params (DeltaSeconds :type Float%20%28single-precision%29)))

(event EventInteraction
  (Utilities|FlowControl|DoOnce false
    (:Completed
      (Development|PrintString "Hello")
      (bind _asbp_third_person_character (Utilities|Casting|CastToBP_ThirdPersonCharacter (Game|GetPlayerCharacter 0)))
      (bind _output_get (Variables|Default|SetMychar _asbp_third_person_character))
      (Variables|/Game/ThirdPerson/Blueprints/BP_ThirdPersonCharacter.BP_ThirdPersonCharacter_C|SetCanDoubleJump _output_get true)
      (Audio|PlaySound2D "/Game/StarterContent/Audio/Explosion_Cue.Explosion_Cue" 1.0 1.0 0.0 0 0)
      (Effects|SpawnEmitteratLocation "/Game/StarterContent/Particles/P_Explosion.P_Explosion" (Transformation|GetSocketLocation (Variables|Default|GetCube) "None")))))

(fn ConstructionScript)

(fn Interact
  (Actor|DestroyActor)
  (return false))